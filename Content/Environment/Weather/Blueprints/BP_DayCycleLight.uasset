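; Day/night cycle light actor that keeps a linked BP_SkySphere and the ambient tint in step with time of day.
; On BeginPlay it hands its directional light to the sky and applies the curve's initial tint, disabling Tick if no sky is found.
; OnTimeChanged plays a curve-driven tint timeline forward for night or backward for day, feeding UpdateAmbient.
; Tick refreshes the sky's sun direction every frame.
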(event `self.ReceiveBeginPlay`
  (`parent.ReceiveBeginPlay`)
  (`self.SetupSky`)
  (add `self.OnTimeChanged` (delegate `StartTint`))
  (`TimelineComponent.SetLinearColorCurve` (`self.TintTimeline`) (`self.TintCurve`) "TintColor"))

(event `StartTint`
  (params (bShouldBeNight :type Boolean))
  ;[1 1 1] Tint Change
  (if bShouldBeNight
    (bind (_direction _tintcolor) (`Timeline|TintTimeline` :!via `PlayFromStart` :!label _label)
      (:`Update`
        (`self.UpdateAmbient` _tintcolor 1.0)))
    (else
      (goto _label :!via `ReverseFromEnd`))))

(event `self.ReceiveTick`
  (params (DeltaSeconds :type "Float (single-precision)"))
  ;[1 1 1] Sky Update
  (`parent.ReceiveTick` DeltaSeconds)
  (bind _asbp_sky_sphere (cast `/Game/Environment/Weather/Blueprints/BP_SkySphere` (`self.SkySphere`)))
  (`/Game/Environment/Weather/Blueprints/BP_SkySphere.UpdateSunDirection` _asbp_sky_sphere))

(fn `ColorEqual`
  (params (Color1 :type "LinearColor Structure") (Color2 :type "LinearColor Structure"))
  (returns (Result :type Boolean))
  (bind (_r _g _b _a) (`KismetMathLibrary.BreakColor` Color1))
  (bind (_r_2 _g_2 _b_2 _a_2) (`KismetMathLibrary.BreakColor` Color2))
  (return (and (== _r _r_2) (== _g _g_2) (== _b _b_2) (== _a _a_2))))

(fn `SetupSky`
  (bind _asbp_sky_sphere (cast `/Game/Environment/Weather/Blueprints/BP_SkySphere` (`self.SkySphere`))
    (:`then`
      (set `/Game/Environment/Weather/Blueprints/BP_SkySphere.Directional light` (`self.DirectionalLight`) _asbp_sky_sphere)
      (`self.UpdateAmbient` (`CurveLinearColor.GetLinearColorValue` (`self.TintCurve`) 0.0) 1.0))
    (:`CastFailed`
      (`self.SetActorTickEnabled` false))))

(fn `UserConstructionScript`)