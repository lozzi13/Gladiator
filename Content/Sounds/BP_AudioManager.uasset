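; BP_AudioManager controls music, ambient and UI audio for a gladiator game.
; Day cycle changes switch day and night music, while rain events swap ambience between wind and intensity-scaled rain.
; A shared ReplaceSound event handles these switches by fading out, swapping the sound and fading back in.
; Game mode win or lose stops ambience, pushes a UI-focus sound mix and plays an end jingle, and OnReset restores the defaults.
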(event `ReplaceSound`
  (params (Audio :type "AudioComponent Object Reference") (NewSound :type "SoundBase Object Reference") (NewVolume :type "Float (double-precision)" :default 1.0) (FadeDuration :type "Float (double-precision)"))
  (bind _returnvalue (/ FadeDuration 2.0))
  ;[1 1 1] Audio Fade
  (if (!= (`AudioComponent.Sound` Audio) NewSound)
    (`AudioComponent.FadeOut` Audio _returnvalue 0.0)
    (`KismetSystemLibrary.Delay` _returnvalue)
    (`AudioComponent.SetSound` Audio NewSound)
    (`AudioComponent.FadeIn` Audio _returnvalue NewVolume 0.0)))

(event `self.Rain.OnRain`
  (params (bIsRaining :type Boolean) (Intensity :type "Float (single-precision)") (Duration :type "Float (single-precision)"))
  (bind _audioambient (`self.AudioAmbient`))
  ;[1 1 1] Ambient Rain
  (if bIsRaining
    (`self.ReplaceSound` _audioambient (`self.RainAmbient`) (+ Intensity 0.5) 2.0)
    (else
      (`self.ReplaceSound` _audioambient (`self.WindAmbient`) 1.0 2.0))))

(event `self.ReceiveBeginPlay`
  (bind _audiomusic (`self.AudioMusic`))
  (bind _daycycle (`self.DayCycle`))
  (`/Engine/EditorBlueprintResources/StandardMacros.IsValid` _daycycle
    (:`Is Valid`
      (add `DayCycleLight.OnTimeChanged` _daycycle (delegate `ChangeMusic`)))
    (:`Is Not Valid`
      _))
  (`AudioComponent.SetSound` _audiomusic "/Game/Sounds/MusicAndAmbient/A_DayMusic.A_DayMusic")
  (`AudioComponent.Play` _audiomusic 0.0)
  ;[1 1 1] Ambient
  (`self.ReplaceSound` (`self.AudioAmbient`) (`self.WindAmbient`) 1.0 1.0)
  (bind _asgladiator_game_mode_base (cast `GladiatorGameModeBase` (`GameplayStatics.GetGameMode`)))
  (add `GladiatorGameModeBase.OnWin` _asgladiator_game_mode_base (delegate `OnGameEnded`))
  (add `GladiatorGameModeBase.OnLose` _asgladiator_game_mode_base (delegate `OnGameEnded`)))

(event `OnGameEnded`
  (bind _audioui (`self.AudioUI`))
  ;[1 1 1] UI
  (`AudioComponent.Stop` (`self.AudioAmbient`))
  (`GameplayStatics.PushSoundMixModifier` "/Game/Sounds/SoundClassesAndMixes/Mix_UIFocus.Mix_UIFocus")
  (`AudioComponent.SetSound` _audioui (`self.EndJingle`))
  (`AudioComponent.Play` _audioui 0.0))

(event `self.K2_OnReset`
  ;[1 1 1] UI
  (`GameplayStatics.PopSoundMixModifier` "/Game/Sounds/SoundClassesAndMixes/Mix_UIFocus.Mix_UIFocus")
  (`self.ReplaceSound` (`self.AudioAmbient`) (`self.WindAmbient`) 1.0 1.0)
  (`self.ChangeMusic` false))

(event `ChangeMusic`
  (params (bShouldBeNight :type Boolean))
  (bind _audiomusic (`self.AudioMusic`))
  ;[1 1 1] Music
  (if bShouldBeNight
    (`self.ReplaceSound` _audiomusic (`self.NightMusic`) 1.0 4.0)
    (else
      (`self.ReplaceSound` _audiomusic (`self.DayMusic`) 1.0 4.0))))

(fn `UserConstructionScript`)