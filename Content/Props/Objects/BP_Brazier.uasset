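; BP_Brazier is a brazier prop that lights at night and goes out by day.
; On BeginPlay it binds LightUp to the DayCycle's time-changed event, if valid, and sets the light to its starting intensity.
; LightUp toggles the particle system and plays or reverses a timeline that fades the point light, scaled by BaseIntensity.
; OnReset turns off the particles and restores the curve's starting intensity.
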(event `self.K2_OnReset`
  (`ActorComponent.Deactivate` (`self.ParticleSystem`))
  ;[1 1 1] Reset intensity
  (`LightComponent.SetIntensity` (`self.PointLight`) (* (`CurveFloat.GetFloatValue` (`self.IntensityCurve`) 0.0) (`self.BaseIntensity`)) :!label _label))

(event `self.ReceiveBeginPlay`
  (bind _daycycle (`self.DayCycle`))
  (`/Engine/EditorBlueprintResources/StandardMacros.IsValid` _daycycle
    (:`Is Valid`
      (add `DayCycleLight.OnTimeChanged` _daycycle (delegate `LightUp`))
      (goto _label))))

(event `LightUp`
  (params (bShouldBeNight :type Boolean))
  ;[1 1 1] OnTimeChanged
  (if bShouldBeNight
    (`ActorComponent.Activate` (`self.ParticleSystem`) true)
    (bind (_direction _intensity) (`Timeline|IntensityTimeline` :!via `PlayFromStart` :!label _label_2)
      (:`Update`
        (`LightComponent.SetIntensity` (`self.PointLight`) (* _intensity (`self.BaseIntensity`)))))
    (else
      (`ActorComponent.Deactivate` (`self.ParticleSystem`))
      (goto _label_2 :!via `ReverseFromEnd`))))

(fn `UserConstructionScript`)