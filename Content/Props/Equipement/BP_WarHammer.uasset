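; BP_WarHammer is a war hammer equipment prop that glows while dropped in the world.
; The construction script assigns the box as its collider and puts a dynamic material instance on the mesh.
; Drop, pick-up and reset events drive that material's emissivity, lighting it up on drop and switching it off when picked up or reset.
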(event `self.OnDropped`
  (`MaterialInstanceDynamic.SetScalarParameterValue` (`self.Material`) "Emissivity" 30.0))

(event `self.K2_OnReset`
  (`MaterialInstanceDynamic.SetScalarParameterValue` (`self.Material`) "Emissivity" 0.0 :!label _label))

(event `self.OnPicked`
  (goto _label))

(fn `UserConstructionScript`
  (bind _mesh (`self.Mesh`))
  (set `self.Collider` (`self.Box`))
  (bind _returnvalue (`PrimitiveComponent.CreateDynamicMaterialInstance` _mesh 0 (`PrimitiveComponent.GetMaterial` (`self.Mesh`) 0)))
  (bind _output_get (set `self.Material` _returnvalue))
  (`PrimitiveComponent.SetMaterial` _mesh 0 _output_get))