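; Game mode for a melee game that shows the win and lose screens when the match ends.
; On BeginPlay it creates both result widgets, adds them to the viewport hidden, and binds handlers to OnWin and OnLose events.
; Either handler reveals its widget, then shares one path that unpossesses the player, shows the cursor and switches to UI-only input.
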(event `self.ReceiveBeginPlay`
  (bind _returnvalue (`GameplayStatics.GetPlayerController` 0))
  ;[1 1 1] Create Widget
  (bind _returnvalue_2 (`|CreateWidget` "/Game/UI/Blueprints/WBP_Win.WBP_Win_C" _returnvalue))
  (bind _output_get (set `self.WinWidget` _returnvalue_2))
  (bind _returnvalue_3 (`|CreateWidget` "/Game/UI/Blueprints/WBP_Lose.WBP_Lose_C" _returnvalue))
  (bind _output_get_2 (set `self.LoseWidget` _returnvalue_3))
  (`UserWidget.AddToViewport` _output_get_2 0)
  (`UserWidget.AddToViewport` _output_get 0)
  (`Widget.SetVisibility` (`self.WinWidget`) "Hidden")
  (`Widget.SetVisibility` (`self.LoseWidget`) "Hidden")
  (add `self.OnWin` (delegate `DisplayWinUI`))
  (add `self.OnLose` (delegate `DisplayLoseUI`)))

(event `DisplayWinUI`
  (bind _returnvalue (`GameplayStatics.GetPlayerController` 0))
  ;[1 1 1] Display Widget
  (`Widget.SetVisibility` (`self.WinWidget`) "Visible")
  ;[1 1 1] Cursor handling
  (`Controller.UnPossess` _returnvalue :!label _label)
  (set `PlayerController.CurrentMouseCursor` "Default" _returnvalue)
  (set `PlayerController.bShowMouseCursor` true _returnvalue)
  (`WidgetBlueprintLibrary.SetInputMode_UIOnlyEx` _returnvalue))

(event `DisplayLoseUI`
  ;[1 1 1] Display Widget
  (`Widget.SetVisibility` (`self.LoseWidget`) "Visible")
  (goto _label))

(fn `UserConstructionScript`)