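; Hero character Blueprint that layers player feedback onto inherited life, hit and death logic.
; Life changes update a health bar as a fraction of MaxLife, and death plays a camera animation, then delays the parent's death handling.
; Hits spawn blood particles whose collisions place blood on surfaces, then after a delay trigger camera shake, sound and a curve-driven timeline reddening two dynamic materials created at construction.
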(event `self.SetLife`
  (params (Value :type "Float (single-precision)"))
  ;[1 1 1] Life Display
  (`parent.SetLife` Value)
  (`self.DisplayLife` Value))

(event `self.ReceiveBeginPlay`
  ;[1 1 1] Life Display
  (`parent.ReceiveBeginPlay`)
  (`self.DisplayLife` (`self.MaxLife`))
  (`TimelineComponent.SetFloatCurve` (`self.HitTimeline`) (`self.HitIntensityCurve`) "Alpha"))

(event `self.OnDeath`
  (`PlayerCameraManager.PlayCameraAnim` :`self` (`GameplayStatics.GetPlayerCameraManager` 0) :`Anim` "/Game/Core/Characters/Hero/CA_Death.CA_Death")
  (`KismetSystemLibrary.Delay` (`self.DeathDelay`))
  (`parent.OnDeath`))

(event `self.OnHit`
  (params (OtherDamage :type Integer))
  (bind _returnvalue (`self.K2_GetActorLocation`))
  (`parent.OnHit` OtherDamage)
  (set `self.bHitOnce` false)
  (if (`self.bHitOnce`) :!label _label
    ;[1 1 1] Hit Feedback
    (bind (_direction _alpha) (`Timeline|HitTimeline` :!via `PlayFromStart`)
      (:`Update`
        (`/Game/Core/Characters/Common/Blueprints/BPFL_Warrior.ReddenMaterial` (`self.Material0`) _alpha)
        (`/Game/Core/Characters/Common/Blueprints/BPFL_Warrior.ReddenMaterial` (`self.Material1`) _alpha)))
    (else
      (set `self.bHitOnce` true)
      ;[1 1 1] Blood Splatter
      (bind _returnvalue_2 (`GameplayStatics.SpawnEmitterAttached` "/Game/Environment/Effects/Particles/PS_Blood.PS_Blood" (`self.Mesh`) "None" (0.0 0.0 100.0)))
      (add `ParticleSystemComponent.OnParticleCollide` _returnvalue_2 (delegate `OnBloodSplatter`))
      ;[1 1 1] Camera Shake + Sound
      (`KismetSystemLibrary.Delay` (`self.CameraShakeDelay`))
      (`GameplayStatics.PlayWorldCameraShake` "/Game/Core/Characters/Hero/BP_CameraShake.BP_CameraShake_C" _returnvalue 0.0 500.0)
      (`GameplayStatics.PlaySoundAtLocation` "/Game/Sounds/Weapons/Metal/A_HitSound_Cue.A_HitSound_Cue" _returnvalue)
      (goto _label))))

(event `OnBloodSplatter`
  (params (EventName :type Name) (EmitterTime :type "Float (double-precision)") (ParticleTime :type Integer) (Location :type "Vector Structure") (Velocity :type "Vector Structure") (Direction :type "Vector Structure") (Normal :type "Vector Structure") (BoneName :type Name) (PhysMat :type "PhysicalMaterial Object Reference"))
  ;[1 1 1] Blood Splatter
  (`/Game/Core/Characters/Common/Blueprints/BPFL_Warrior.SpawnBlood` self 50.0 75.0 Location Normal))

(fn `DisplayLife`
  (params (Life :type "Float (double-precision)"))
  (bind _healthbar (`self.HealthBar`))
  (`/Engine/EditorBlueprintResources/StandardMacros.IsValid` _healthbar
    (:`Is Valid`
      (`ProgressBar.SetPercent` _healthbar (/ Life (`self.MaxLife`))))))

(fn `UserConstructionScript`
  (bind _mesh (`self.Mesh`))
  (bind _returnvalue (`PrimitiveComponent.CreateDynamicMaterialInstance` _mesh 0 (`PrimitiveComponent.GetMaterial` _mesh 0)))
  (set `self.Material0` _returnvalue)
  (bind _returnvalue_2 (`PrimitiveComponent.CreateDynamicMaterialInstance` _mesh 1 (`PrimitiveComponent.GetMaterial` _mesh 1)))
  (set `self.Material1` _returnvalue_2))