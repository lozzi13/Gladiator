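; Enemy character Blueprint that adds health display, hit feedback and a lock-on marker to its parent's life, hit and death events.
; Life changes update a widget health bar, which collapses with the arrow after a death delay.
; Hits play a sound, emit blood that spawns splatters on particle collision, and redden two dynamic materials through a curve-driven timeline.
; While locked, a second timeline animates the arrow's location and rotation.
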(event `self.ReceiveBeginPlay`
  (`parent.ReceiveBeginPlay`)
  (bind _aswbp_enemy_hud (cast `/Game/UI/Blueprints/WBP_EnemyHUD` (`WidgetComponent.GetUserWidgetObject` (`self.Health`))))
  (set `self.HealthBar` (`/Game/UI/Blueprints/WBP_EnemyHUD.HealthBar` _aswbp_enemy_hud))
  (`self.DisplayLife` (`self.MaxLife`))
  (`TimelineComponent.SetFloatCurve` (`self.HitTimeline`) (`self.HitIntensityCurve`) "Alpha")
  (`SceneComponent.SetVisibility` (`self.LockedArrow`) false false))

(event `self.OnDeath`
  (`KismetSystemLibrary.Delay` (`self.DeathDelay`))
  (`Widget.SetVisibility` (`self.HealthBar`) "Collapsed")
  (`SceneComponent.SetVisibility` (`self.LockedArrow`) false false)
  (`parent.OnDeath`))

(event `self.SetLife`
  (params (Value :type "Float (single-precision)"))
  (`parent.SetLife` Value)
  (`self.DisplayLife` Value))

(event `self.OnHit`
  (params (OtherDamage :type Integer))
  (`parent.OnHit` OtherDamage)
  (`GameplayStatics.PlaySoundAtLocation` "/Game/Sounds/Weapons/Metal/A_HitSound_Cue.A_HitSound_Cue" (`self.K2_GetActorLocation`))
  (bind _returnvalue (`GameplayStatics.SpawnEmitterAttached` "/Game/Environment/Effects/Particles/PS_Blood.PS_Blood" (`self.Mesh`) "None" (0.0 0.0 100.0)))
  (add `ParticleSystemComponent.OnParticleCollide` _returnvalue (delegate `OnBloodSplatter`))
  (bind (_direction _alpha) (`Timeline|HitTimeline` :!via `PlayFromStart`)
    (:`Update`
      (`/Game/Core/Characters/Common/Blueprints/BPFL_Warrior.ReddenMaterial` (`self.Material0`) _alpha)
      (`/Game/Core/Characters/Common/Blueprints/BPFL_Warrior.ReddenMaterial` (`self.Material1`) _alpha))))

(event `OnBloodSplatter`
  (params (EventName :type Name) (EmitterTime :type "Float (double-precision)") (ParticleTime :type Integer) (Location :type "Vector Structure") (Velocity :type "Vector Structure") (Direction :type "Vector Structure") (Normal :type "Vector Structure") (BoneName :type Name) (PhysMat :type "PhysicalMaterial Object Reference"))
  (`/Game/Core/Characters/Common/Blueprints/BPFL_Warrior.SpawnBlood` self 50.0 75.0 Location Normal))

(event `self.OnLock`
  (bind _lockedarrow (`self.LockedArrow`))
  (bind _lockedarrow_2 (`self.LockedArrow`))
  (if (`self.bIsLocked`)
    (`SceneComponent.SetVisibility` _lockedarrow true false)
    (bind (_direction _location _rotation) (`Timeline|ArrowTimeline` :!label _label)
      (:`Update`
        (`SceneComponent.K2_SetRelativeLocation` _lockedarrow_2 _location false false)
        (`SceneComponent.K2_SetRelativeRotation` _lockedarrow_2 (`KismetMathLibrary.MakeRotator` (.x _rotation) (.y _rotation) (.z _rotation)) false false)))
    (else
      (`SceneComponent.SetVisibility` _lockedarrow false false)
      (goto _label :!via `Stop`))))

(fn `DisplayLife`
  (params (Life :type "Float (double-precision)"))
  (bind _healthbar (`self.HealthBar`))
  (`/Engine/EditorBlueprintResources/StandardMacros.IsValid` _healthbar
    (:`Is Valid`
      (`ProgressBar.SetPercent` _healthbar (/ Life (`self.MaxLife`))))))

(fn `UserConstructionScript`
  (bind _mesh (`self.Mesh`))
  (bind _returnvalue (`PrimitiveComponent.CreateDynamicMaterialInstance` _mesh 0 (`PrimitiveComponent.GetMaterial` _mesh 0)))
  (set `self.Material0` _returnvalue)
  (bind _returnvalue_2 (`PrimitiveComponent.CreateDynamicMaterialInstance` _mesh 1 (`PrimitiveComponent.GetMaterial` _mesh 1)))
  (set `self.Material1` _returnvalue_2))